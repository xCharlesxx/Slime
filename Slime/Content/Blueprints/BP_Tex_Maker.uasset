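; BP_Tex_Maker is a controller actor that paints branching, slime-like growth into the RT_Whiteboard render target.
; On BeginPlay it creates a dynamic material, clears the target and hands the material to RTManipulation actors, then draws it to the target every tick.
; Draw events send locations to RTManipulation's BranchTowards.
; Debug keys tune and print branching parameters, clear the slime, restart the level or quit.
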(event Custom|Bake)

(event Custom|Draw
  (params (Location%20to%20Draw :type Vector%202D%20Structure))
  (Class|RTManipulation|BranchTowards (stale EventBeginPlay _asrtmanipulation) Location%20to%20Draw))

(event EventTick
  (params (DeltaSeconds :type Float%20%28single-precision%29))
  (Rendering|DrawMaterialtoRenderTarget "/Game/WhiteBoard/RT_Whiteboard.RT_Whiteboard" (Variables|Default|GetMaterialInstanceDynamic)))

(event EventBeginPlay
  (Input|EnableInput (Game|GetPlayerController 0))
  (bind _returnvalue (Rendering|Material|CreateDynamicMaterialInstance "/Game/Blueprints/DMatParent.DMatParent" "None" :!class /Script/Engine.KismetMaterialLibrary))
  (bind _output_get (Variables|Default|SetMaterialInstanceDynamic _returnvalue))
  (Rendering|ClearRenderTarget2D "/Game/WhiteBoard/RT_Whiteboard.RT_Whiteboard")
  (bind _outactors (Actor|GetAllActorsOfClass "/Script/Slime.RTManipulation"))
  (for _array_element _outactors
    (bind _asrtmanipulation (Utilities|Casting|CastToRTManipulation _array_element))
    (Class|RTManipulation|SetDynamicMat _asrtmanipulation _output_get)
    (Variables|Default|SetSegLength 3)
    (Variables|Default|SetBranchProb 0.3)
    (Variables|Default|SetGenPen 0.01)
    (Variables|Default|SetSpeed 0.05)
    (Variables|Default|SetMaxBranch 20)
    (Class|RTManipulation|UpdateParams _asrtmanipulation (stale Input|KeyboardEvents|Y _output_get) (stale Input|KeyboardEvents|U _output_get) (stale Input|KeyboardEvents|I _output_get) (stale Input|KeyboardEvents|O _output_get) (stale Input|KeyboardEvents|T _output_get))))

(event Input|KeyboardEvents|SpaceBar
  (params (Key :type Key%20Structure))
  (:Pressed
    (Class|RTManipulation|ClearSlime (stale EventBeginPlay _asrtmanipulation))))

(event Input|KeyboardEvents|Y
  (params (Key :type Key%20Structure))
  (:Pressed
    (bind _output_get (Variables|Default|SetSegLength (+ (Variables|Default|GetSegLength) 1)))
    (Development|PrintString (Utilities|String|BuildString(Integer) "Segment Length: " "" (stale Input|KeyboardEvents|H _output_get)))
    (Class|RTManipulation|UpdateParams (stale EventBeginPlay _asrtmanipulation) _output_get (stale Input|KeyboardEvents|U _output_get) (stale Input|KeyboardEvents|I _output_get) (stale Input|KeyboardEvents|O _output_get) (stale Input|KeyboardEvents|T _output_get))))

(event Input|KeyboardEvents|G
  (params (Key :type Key%20Structure))
  (:Pressed
    (bind _output_get (Variables|Default|SetMaxBranch (- (Variables|Default|GetMaxBranch) 1)))
    (Development|PrintString (Utilities|String|BuildString(Integer) "Max Branches: " "" _output_get))
    (Class|RTManipulation|UpdateParams (stale EventBeginPlay _asrtmanipulation) (stale Input|KeyboardEvents|Y _output_get) (stale Input|KeyboardEvents|U _output_get) (stale Input|KeyboardEvents|I _output_get) (stale Input|KeyboardEvents|O _output_get) (stale Input|KeyboardEvents|T _output_get))))

(event Input|KeyboardEvents|Escape
  (params (Key :type Key%20Structure))
  (:Pressed
    (Game|QuitGame 0 "Quit" true)))

(event Input|KeyboardEvents|R
  (params (Key :type Key%20Structure))
  (:Pressed
    (Development|ExecuteConsoleCommand "restartlevel" 0)))

(event Input|KeyboardEvents|H
  (params (Key :type Key%20Structure))
  (:Pressed
    (bind _output_get (Variables|Default|SetSegLength (- (Variables|Default|GetSegLength) 1)))
    (Development|PrintString (Utilities|String|BuildString(Integer) "Segment Length: " "" _output_get))
    (Class|RTManipulation|UpdateParams (stale EventBeginPlay _asrtmanipulation) (stale Input|KeyboardEvents|Y _output_get) (stale Input|KeyboardEvents|U _output_get) (stale Input|KeyboardEvents|I _output_get) (stale Input|KeyboardEvents|O _output_get) (stale Input|KeyboardEvents|T _output_get))))

(event Input|KeyboardEvents|U
  (params (Key :type Key%20Structure))
  (:Pressed
    (bind _output_get (Variables|Default|SetBranchProb (+ (Variables|Default|GetBranchProb) 0.1)))
    (Development|PrintString (Utilities|String|BuildString(Float) "Branch Probability: " "" (stale Input|KeyboardEvents|J _output_get)))
    (Class|RTManipulation|UpdateParams (stale EventBeginPlay _asrtmanipulation) (stale Input|KeyboardEvents|Y _output_get) _output_get (stale Input|KeyboardEvents|I _output_get) (stale Input|KeyboardEvents|O _output_get) (stale Input|KeyboardEvents|T _output_get))))

(event Input|KeyboardEvents|J
  (params (Key :type Key%20Structure))
  (:Pressed
    (bind _output_get (Variables|Default|SetBranchProb (- (Variables|Default|GetBranchProb) 0.1)))
    (Development|PrintString (Utilities|String|BuildString(Float) "Branch Probability: " "" _output_get))
    (Class|RTManipulation|UpdateParams (stale EventBeginPlay _asrtmanipulation) (stale Input|KeyboardEvents|Y _output_get) (stale Input|KeyboardEvents|U _output_get) (stale Input|KeyboardEvents|I _output_get) (stale Input|KeyboardEvents|O _output_get) (stale Input|KeyboardEvents|T _output_get))))

(event Input|KeyboardEvents|I
  (params (Key :type Key%20Structure))
  (:Pressed
    (bind _output_get (Variables|Default|SetGenPen (+ (Variables|Default|GetGenPen) 0.1)))
    (Development|PrintString (Utilities|String|BuildString(Float) "Generation Penalty: " "" (stale Input|KeyboardEvents|K _output_get)))
    (Class|RTManipulation|UpdateParams (stale EventBeginPlay _asrtmanipulation) (stale Input|KeyboardEvents|Y _output_get) (stale Input|KeyboardEvents|U _output_get) _output_get (stale Input|KeyboardEvents|O _output_get) (stale Input|KeyboardEvents|T _output_get))))

(event Input|KeyboardEvents|K
  (params (Key :type Key%20Structure))
  (:Pressed
    (bind _output_get (Variables|Default|SetGenPen (- (Variables|Default|GetGenPen) 0.1)))
    (Development|PrintString (Utilities|String|BuildString(Float) "Generation Penalty: " "" _output_get))
    (Class|RTManipulation|UpdateParams (stale EventBeginPlay _asrtmanipulation) (stale Input|KeyboardEvents|Y _output_get) (stale Input|KeyboardEvents|U _output_get) (stale Input|KeyboardEvents|I _output_get) (stale Input|KeyboardEvents|O _output_get) (stale Input|KeyboardEvents|T _output_get))))

(event Input|KeyboardEvents|O
  (params (Key :type Key%20Structure))
  (:Pressed
    (bind _output_get (Variables|Default|SetSpeed (+ (Variables|Default|GetSpeed) 0.01)))
    (Development|PrintString (Utilities|String|BuildString(Float) "Speed:  " "" (stale Input|KeyboardEvents|L _output_get)))
    (Class|RTManipulation|UpdateParams (stale EventBeginPlay _asrtmanipulation) (stale Input|KeyboardEvents|Y _output_get) (stale Input|KeyboardEvents|U _output_get) (stale Input|KeyboardEvents|I _output_get) _output_get (stale Input|KeyboardEvents|T _output_get))))

(event Input|KeyboardEvents|L
  (params (Key :type Key%20Structure))
  (:Pressed
    (bind _output_get (Variables|Default|SetSpeed (- (Variables|Default|GetSpeed) 0.01)))
    (Development|PrintString (Utilities|String|BuildString(Float) "Speed:  " "" _output_get))
    (Class|RTManipulation|UpdateParams (stale EventBeginPlay _asrtmanipulation) (stale Input|KeyboardEvents|Y _output_get) (stale Input|KeyboardEvents|U _output_get) (stale Input|KeyboardEvents|I _output_get) (stale Input|KeyboardEvents|O _output_get) (stale Input|KeyboardEvents|T _output_get))))

(event Input|KeyboardEvents|T
  (params (Key :type Key%20Structure))
  (:Pressed
    (bind _output_get (Variables|Default|SetMaxBranch (+ (Variables|Default|GetMaxBranch) 1)))
    (Development|PrintString (Utilities|String|BuildString(Integer) "Max Branches: " "" (stale Input|KeyboardEvents|G _output_get)))
    (Class|RTManipulation|UpdateParams (stale EventBeginPlay _asrtmanipulation) (stale Input|KeyboardEvents|Y _output_get) (stale Input|KeyboardEvents|U _output_get) (stale Input|KeyboardEvents|I _output_get) (stale Input|KeyboardEvents|O _output_get) _output_get)))

(fn ConstructionScript
  (CallFunction|Bake))